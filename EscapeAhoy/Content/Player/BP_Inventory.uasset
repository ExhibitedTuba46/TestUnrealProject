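; BP_Inventory is a player inventory that stores items in a slot array and tracks whether it is full.
; CollectItem puts CurrentItem in the first empty slot, setting the full flag when that slot is index 4.
; DropItem clears slots matching SelectedItem and resets the flag.
; InventoryItemSelected only prints the selected item's slot index.
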(event Custom|CollectItem
  (bind _inventoryslots (Variables|Default|GetInventorySlots))
  (bind (_array_element _array_index) (Utilities|Array|ForEachLoopwithBreak _inventoryslots :!label _label)
    (:LoopBody
      (Utilities|IsValid _array_element
        (:Is%20Not%20Valid
          (if (== _array_index 4)
            (Variables|Default|SetIsInventoryFull true))
          (Utilities|Array|SetArrayElem _inventoryslots _array_index (Variables|Default|GetCurrentItem))
          (goto _label Break))))))

(event Custom|InventoryItemSelected
  (Development|PrintString (Utilities|String|ToString(Integer) (Utilities|Array|FindItem (Variables|Default|GetInventorySlots) (Variables|Default|GetSelectedItem)))))

(event Custom|DropItem
  (for (_array_element _array_index) (Variables|Default|GetInventorySlots)
    (if (== _array_element (Variables|Default|GetSelectedItem))
      (Utilities|Array|SetArrayElem (Variables|Default|GetInventorySlots) _array_index 0)
      (Variables|Default|SetIsInventoryFull false))))

(fn ConstructionScript)