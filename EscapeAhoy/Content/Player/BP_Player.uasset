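; Player Blueprint for point-and-click interaction, with a camera that turns in steps and can zoom.
; Turn events drive actor yaw through timelines, removing all widgets during the turn and recreating the turn buttons afterward; they assume 90-degree alignment.
; Left click traces from camera through cursor, calling OnSelect on any BP_SelectableObject hit.
; ZoomCamera toggles a flag that makes Tick interpolate from the stored camera position toward CameraZoomPosition.
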(event Custom|ZoomCamera
  (Variables|Default|SetInitialCameraPosition (Transformation|GetWorldLocation (Variables|Default|GetCamera)))
  (if (Variables|Default|GetIsZoomingCamera)
    (Variables|Default|SetIsZoomingCamera false)
    (else
      (Variables|Default|SetIsZoomingCamera true))))

(event Custom|Rotate%20Camera%20Right
  ;[0.149 0.149 0.149] Rotate the player to the right (if not synced up with 90 degree intervals this will break)
  ;;[0.149 0.149 0.149] Get the current rotation of the player
  (Variables|Default|SetinitialRotation (Transformation|GetActorRotation))
  ;;[0.149 0.149 0.149] Rotate the player based on the current rotation of the player and the timeline
  (bind _newtrack_0 (Timeline|Turn%20Right PlayFromStart)
    (:Update
      (Viewport|RemoveAllWidgets)
      (Transformation|SetActorRotation (Math|Rotator|MakeRotator 0.0 0.0 (+ (.Yaw (Math|Rotator|BreakRotator (Variables|Default|GetinitialRotation))) _newtrack_0)) true))
    (:Finished
      (CallFunction|EnableCameraRotationUIButtons))))

(event Custom|Rotate%20Camera%20Left
  ;[0.149 0.149 0.149] Rotate the player to the left (if not synced up with 90 degree intervals this will break)
  ;;[0.149 0.149 0.149] Get the current rotation of the player
  (Variables|Default|SetinitialRotation (Transformation|GetActorRotation))
  ;;[0.149 0.149 0.149] Rotate the player based on the current rotation of the player and the timeline
  (bind _newtrack_0 (Timeline|Turn%20Left PlayFromStart)
    (:Update
      (Viewport|RemoveAllWidgets)
      (Transformation|SetActorRotation (Math|Rotator|MakeRotator 0.0 0.0 (+ (.Yaw (Math|Rotator|BreakRotator (Variables|Default|GetinitialRotation))) _newtrack_0)) true))
    (:Finished
      (CallFunction|EnableCameraRotationUIButtons))))

(event EventBeginPlay
  ;[0.15 0.15 0.15 0.5] Initial variable setup
  (CallFunction|EnableCameraRotationUIButtons)
  (Variables|Default|SetInitialCameraPosition (Transformation|GetWorldLocation (Variables|Default|GetCamera))))

(event EventTick
  (params (DeltaSeconds :type Float%20%28single-precision%29))
  (if (Variables|Default|GetIsZoomingCamera)
    (Transformation|SetWorldLocation (Variables|Default|GetCamera) (Math|Interpolation|VInterpTo (Variables|Default|GetInitialCameraPosition) (Variables|Default|GetCameraZoomPosition) DeltaSeconds 0.0) false false)))

(event Input|MouseEvents|LeftMouseButton
  (params (Key :type Key%20Structure :default "None"))
  (bind _returnvalue (Game|GetPlayerController 0))
  (bind (_worldlocation _worlddirection) (Game|Player|ConvertMouseLocationToWorldSpace _returnvalue))
  ;[0.15 0.15 0.15 0.5] When the left mouse button is pressed create a raycast from the camera to the mouse's position, and select an object
  (:Pressed
    (bind _outhit (Collision|LineTraceByChannel (Transformation|GetWorldLocation (Variables|Default|GetCamera)) (+ _worldlocation (* _worlddirection 1e+03)) "TraceTypeQuery1" false 0 "Persistent"))
    ;;[0.15 0.15 0.15 0.5] If the object that collides with the ray is a point of interest then trigger it
    (bind _asbp_selectable_object (Utilities|Casting|CastToBP_SelectableObject (.HitActor (Collision|BreakHitResult _outhit))))
    (Default|OnSelect _asbp_selectable_object)))

(fn ConstructionScript)

(fn EnableCameraRotationUIButtons
  (bind _returnvalue (UserInterface|CreateWidget "/Game/UserInterface/BP_LeftTurnButton.BP_LeftTurnButton_C"))
  (UserInterface|Viewport|AddtoViewport _returnvalue 0)
  (bind _returnvalue_2 (UserInterface|CreateWidget "/Game/UserInterface/BP_RIghtTurnButton.BP_RIghtTurnButton_C"))
  (UserInterface|Viewport|AddtoViewport _returnvalue_2 0))