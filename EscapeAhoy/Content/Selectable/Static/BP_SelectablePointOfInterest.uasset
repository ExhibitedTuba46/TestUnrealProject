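; Selectable point of interest that zooms the player camera in on it when selected.
; OnSelect acts only if BP_Player is not zoomed and its rotation matches RotationRequirement, then triggers the zoom, passes the CameraZoomPosition location and calls the empty OnSelectAdditional hook.
; Helper functions move PuzzleElements to their interaction locations or to a fixed removal spot, but their calls in the event graph are unconnected.
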(event Custom|OnSelectAdditional
  ;[0.15 0.15 0.15 0.5] Abstract events
)

(event Custom|OnDeSelect
  ;[0.15 0.15 0.15 0.5] Abstract events
)

(event EventOnSelect
  ;[0.15 0.15 0.15 0.5] When selected trigger the camera to zoom
  (bind _returnvalue (Actor|GetActorOfClass "/Game/Player/BP_Player.BP_Player_C"))
  (if (not (Variables|/Game/Player/BP_Player.BP_Player_C|GetIsCameraZoomed _returnvalue))
    (if (Utilities|Operators|EqualEqual (Transformation|GetActorRotation _returnvalue) (Math|Rotator|MakeRotator 0.0 0.0 (Variables|Default|GetRotationRequirement)) 0.0)
      (Default|ZoomCamera _returnvalue)
      ;[0.15 0.15 0.15 0.5] Call additional functionality if needed
      (Variables|/Game/Player/BP_Player.BP_Player_C|SetCameraZoomPosition _returnvalue (Transformation|GetWorldLocation (Variables|Default|GetCameraZoomPosition)))
      (CallFunction|OnSelectAdditional))))

(fn ConstructionScript
  (|CallParentFunction))

(fn RemovePuzzleElements
  (for _array_element (Variables|Default|GetPuzzleElements)
    (Transformation|SetActorLocation _array_element "0.000000,-10.000000,0.000000" false false)))

(fn AddPuzzleElements
  (for _array_element (Variables|Default|GetPuzzleElements)
    (Transformation|SetActorLocation _array_element (Variables|/Game/Selectable/Static/BP_ItemInteractionSpot.BP_ItemInteractionSpot_C|GetIneractionLocation _array_element) false false)))