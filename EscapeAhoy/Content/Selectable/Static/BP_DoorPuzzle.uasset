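; Selectable door with a five-row combination lock that ends the game when solved.
; Selection adds puzzle elements; Tick polls ten of them as left/right triggers, rotating rows and updating RowStates, with uneven steps and fixed wraparound rotations for off-center digits.
; Tick also compares RowStates to DoorCombination; a match deselects the door, calls GameEnd on BP_Player, swings the hinge open by Timeline and shows the win screen.
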(event EventBeginPlay
  ;[0.15 0.15 0.15 0.5] Puzzle element control
  (Utilities|FlowControl|Delay 0.2)
  (CallFunction|RemovePuzzleElements)
  (Variables|Default|SetInitialRowRotation (Transformation|GetWorldRotation (Variables|Default|GetRow1))))

(event EventTick
  (params (DeltaSeconds :type Float%20%28single-precision%29))
  ;[0.15 0.15 0.15 0.5] Check whether the door currently has the correct code
  (Variables|Default|SetDelta%20Seconds DeltaSeconds)
  (Variables|Default|SetPuzzleComplete true)
  (for (_array_element _array_index) (Variables|Default|GetRowStates)
    ;[0.15 0.15 0.15 0.5] If the combination in the Door Combination variable is the same as the current state of the lock
    (if (!= _array_element (Utilities|Array|Get(acopy) (Variables|Default|GetDoorCombination) _array_index))
      (Variables|Default|SetPuzzleComplete false)))
  (if (Variables|Default|GetPuzzleComplete)
    ;[0.15 0.15 0.15 0.5] De-select the door and end the game in the player blueprint
    (Actor|GetActorOfClass "/Game/Player/BP_Player.BP_Player_C")
    (CallFunction|OnDeSelect)
    (Utilities|FlowControl|DoOnce false
      (:Completed
        (bind _returnvalue (Actor|GetActorOfClass "/Game/Player/BP_Player.BP_Player_C"))
        (Default|GameEnd _returnvalue)
        ;[0.15 0.15 0.15 0.5] Rotate the door to open up
        (Utilities|FlowControl|Delay 2.0)
        (bind _rotation (Timeline|Timeline PlayFromStart)
          (:Update
            (Transformation|SetWorldRotation (Variables|Default|GetDoorHinge) (Math|Rotator|MakeRotator 0.0 0.0 _rotation) false false))
          (:Finished
            ;[0.15 0.15 0.15 0.5] Create a winscreen UI window
            (Utilities|FlowControl|Delay 1.0)
            (bind _returnvalue_2 (UserInterface|CreateWidget "/Game/UserInterface/Menu/W_Winscreen.W_Winscreen_C"))
            (UserInterface|Viewport|AddtoViewport _returnvalue_2 0)))))
    (else
      ;[0.15 0.15 0.15 0.5] There is definitely a more efficient way to do this, but I am running low on time and I just want it to work
      (Utilities|FlowControl|Sequence
        (:then_0
          (|CollapseGraph :!label _label))
        (:then_1
          (goto _label execute2))
        (:then_2
          (goto _label execute3))
        (:then_3
          (goto _label execute4))
        (:then_4
          (goto _label execute5))
        (:then_5
          (goto _label execute6))
        (:then_6
          (goto _label execute7))
        (:then_7
          (goto _label execute8))
        (:then_8
          (goto _label execute9))
        (:then_9
          (goto _label execute10))))))

(event EventOnSelectAdditional
  ;[0.15 0.15 0.15 0.5] Puzzle element control
  (CallFunction|AddPuzzleElements))

(event EventOnDeSelect
  ;[0.15 0.15 0.15 0.5] Puzzle element control
  (CallFunction|RemovePuzzleElements))

(fn ConstructionScript
  (|CallParentFunction))

(fn GetInteractorIndex
  (params (index :type Integer))
  ;[0.15 0.15 0.15 0.5] Get the index of a puzzle element
  (return (Variables|/Game/Selectable/Static/BP_ItemInteractionSpot.BP_ItemInteractionSpot_C|GetItemPlaced (Utilities|Array|Get(acopy) (Variables|Default|GetPuzzleElements) index))))

(fn ResetInteractor
  (for _array_element (Variables|Default|GetPuzzleElements)
    (Default|ResetInteractionCollider _array_element)))

(fn RotateRow
  (params (Row :type Static%20Mesh%20Component%20Object%20Reference) (RotatrionAmount :type Integer) (Index :type Integer))
  (bind _rowstates (Variables|Default|GetRowStates))
  ;[0.15 0.15 0.15 0.5] Rotate the given object by the given value
  (Transformation|SetWorldRotation Row (Math|Rotator|MakeRotator 0.0 0.0 (+ (.Yaw (Math|Rotator|BreakRotator (Transformation|GetWorldRotation Row))) RotatrionAmount)) false false)
  (CallFunction|AddPuzzleElements)
  (Utilities|Array|SetArrayElem _rowstates Index (+ (Utilities|Array|Get(acopy) _rowstates Index) 1)))

(fn RotateRight
  (params (Index :type Integer) (PuzzleIndex :type Integer) (NewParam :type Static%20Mesh%20Component%20Object%20Reference))
  (bind _rowstates (Variables|Default|GetRowStates))
  (bind _output (Utilities|Array|Get(acopy) _rowstates Index))
  ;[0.15 0.15 0.15 0.5] Reset the current interactor
  (bind _itemplaced (CallFunction|GetInteractorIndex PuzzleIndex))
  (if _itemplaced
    (CallFunction|ResetInteractor)
    (CallFunction|RemovePuzzleElements)
    ;[0.15 0.15 0.15 0.5] If the number on the lock is currently <= than 7 rotate by 35 degrees
    (if (<= _output 7)
      (CallFunction|RotateRow NewParam 35 Index)
      (else
        ;[0.15 0.15 0.15 0.5] If the number on the lock currently = 8 then rotate by 40 degrees
        (if (== _output 8)
          (CallFunction|RotateRow NewParam 40 Index)
          (else
            ;[0.15 0.15 0.15 0.5] If the number on the lock currently = 9 then reset rotation to the rotation 9 is located at, as it is slightly off-center
            (if (== _output 9)
              (Transformation|SetWorldRotation NewParam (Variables|Default|GetInitialRowRotation) false false)
              (Utilities|Array|SetArrayElem (Variables|Default|GetRowStates) Index 0)
              (CallFunction|AddPuzzleElements))))))))

(fn RotateLeft
  (params (Index :type Integer) (PuzzleIndex :type Integer) (NewParam :type Static%20Mesh%20Component%20Object%20Reference))
  (bind _rowstates (Variables|Default|GetRowStates))
  (bind _output (Utilities|Array|Get(acopy) _rowstates Index))
  ;[0.15 0.15 0.15 0.5] Reset the current interactor
  (bind _itemplaced (CallFunction|GetInteractorIndex PuzzleIndex))
  (if _itemplaced
    (CallFunction|ResetInteractor)
    (CallFunction|RemovePuzzleElements)
    ;[0.15 0.15 0.15 0.5] If the number on the lock currently >= than 1 but is also < than 9 then rotate by -35 degrees
    (if (and (>= _output 1) (< _output 9))
      (CallFunction|RotateRowBack NewParam -35 Index)
      (else
        ;[0.15 0.15 0.15 0.5] If the number on the lock currently = 9 then rotate by -40 degrees
        (if (== _output 9)
          (CallFunction|RotateRowBack NewParam -40 Index)
          (else
            ;[0.15 0.15 0.15 0.5] If the number on the lock currently = 0 then reset the rotation to where 0 is located becaus 9 is slightly off-center
            (if (== _output 0)
              (Transformation|SetWorldRotation NewParam "0.000000,-130.000000,0.000000" false false)
              (Utilities|Array|SetArrayElem (Variables|Default|GetRowStates) Index 9)
              (CallFunction|AddPuzzleElements))))))))

(fn RotateRowBack
  (params (Row :type Static%20Mesh%20Component%20Object%20Reference) (RotatrionAmount :type Integer) (Index :type Integer))
  (bind _rowstates (Variables|Default|GetRowStates))
  ;[0.15 0.15 0.15 0.5] Rotate the given object by the given value
  (Transformation|SetWorldRotation Row (Math|Rotator|MakeRotator 0.0 0.0 (+ (.Yaw (Math|Rotator|BreakRotator (Transformation|GetWorldRotation Row))) RotatrionAmount)) false false)
  (CallFunction|AddPuzzleElements)
  (Utilities|Array|SetArrayElem _rowstates Index (- (Utilities|Array|Get(acopy) _rowstates Index) 1)))