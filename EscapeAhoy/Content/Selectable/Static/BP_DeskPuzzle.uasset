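; BP_DeskPuzzle is a selectable desk puzzle that opens a drawer once an item is placed in its spot.
; Selecting the desk adds the puzzle elements; deselecting removes them, as does BeginPlay after a short delay before caching the drawer's start location.
; Tick polls the first element until its item is placed, then marks the puzzle complete and plays a timeline that lerps the drawer to the Cube component's location.
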(event EventBeginPlay
  ;[0.15 0.15 0.15 0.5] Set intial states for the desk
  (Utilities|FlowControl|Delay 0.2)
  (CallFunction|RemovePuzzleElements)
  (Variables|Default|SetIntialDrawLocation (Transformation|GetWorldLocation (Variables|Default|GetSM_Desk_Drawer1))))

(event EventTick
  (params (DeltaSeconds :type Float%20%28single-precision%29))
  ;[0.15 0.15 0.15 0.5] If the desk puzzle is marked as complete, lerp the draw's location to the open position.
  (if (not (Variables|Default|GetPuzzleComplete))
    (if (Variables|/Game/Selectable/Static/BP_ItemInteractionSpot.BP_ItemInteractionSpot_C|GetItemPlaced (Utilities|Array|Get(acopy) (Variables|Default|GetPuzzleElements)))
      (Variables|Default|SetPuzzleComplete true)
      (bind _newtrack_0 (Timeline|OpenDraw%28I%20think%20thats%20how%20you%20spell%20it%29 PlayFromStart)
        (:Update
          (Transformation|SetWorldLocation (Variables|Default|GetSM_Desk_Drawer1) (Math|Vector|Lerp(Vector) (Variables|Default|GetIntialDrawLocation) (Transformation|GetWorldLocation (Variables|Default|GetCube)) _newtrack_0) false false))))))

(event EventOnSelectAdditional
  ;[0.15 0.15 0.15 0.5] When the desk is selected add the item spots
  (CallFunction|AddPuzzleElements))

(event EventOnDeSelect
  ;[0.15 0.15 0.15 0.5] When the desk is no longer selected remove item spots
  (CallFunction|RemovePuzzleElements))

(fn ConstructionScript
  (|CallParentFunction))