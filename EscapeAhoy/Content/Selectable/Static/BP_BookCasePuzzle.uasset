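; Selectable bookcase puzzle that swings open its door once every puzzle element has an item placed.
; Selecting it moves the elements to their interaction locations; deselecting, or a short delay after BeginPlay, moves them all to one out-of-the-way position.
; Tick polls each element into a placed-state array until all are true, then a timeline drives the door's yaw.
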(event EventTick
  (params (DeltaSeconds :type Float%20%28single-precision%29))
  (if (not (Variables|Default|GetPuzzleCompleted))
    (for (_array_element _array_index) (Variables|Default|GetPuzzleElements)
      (if (Variables|/Game/Selectable/Static/BP_ItemInteractionSpot.BP_ItemInteractionSpot_C|GetItemPlaced _array_element)
        (Utilities|Array|SetArrayElem (Variables|Default|GetItemsPlaced) _array_index true)))
    (Variables|Default|SetPuzzleCompleted true)
    (for _array_element_2 (Variables|Default|GetItemsPlaced)
      (if (not _array_element_2)
        (Variables|Default|SetPuzzleCompleted false)))
    (if (Variables|Default|GetPuzzleCompleted)
      (bind _rotation (Timeline|OpenDoor PlayFromStart)
        (:Update
          (Transformation|SetWorldRotation (Variables|Default|GetSM_BookcaseDoor) (Math|Rotator|MakeRotator 0.0 0.0 _rotation) false false))))))

(event EventOnSelectAdditional
  (for _array_element (Variables|Default|GetPuzzleElements)
    (Transformation|SetActorLocation _array_element (Variables|/Game/Selectable/Static/BP_ItemInteractionSpot.BP_ItemInteractionSpot_C|GetIneractionLocation _array_element) false false)))

(event EventBeginPlay
  (Utilities|FlowControl|Delay 0.2)
  (CallFunction|RemovePuzzleElements))

(event EventOnDeSelect
  (CallFunction|RemovePuzzleElements))

(fn ConstructionScript
  (|CallParentFunction))

(fn RemovePuzzleElements
  (for _array_element (Variables|Default|GetPuzzleElements)
    (Transformation|SetActorLocation _array_element "0.000000,-10.000000,0.000000" false false)))