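; Selectable painting puzzle in which using one of two interactors turns the Queen Vic painting over by 180 degrees.
; Selection adds the interactors while the puzzle is unsolved, and deselection removes them.
; Tick polls both elements' ItemPlaced flags, and either one completes the puzzle and removes the interactors.
; Timelines then lerp the painting forward to PaintingMoveTo while rotating it right or left, then back to its starting position.
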(event EventTick
  (params (DeltaSeconds :type Float%20%28single-precision%29))
  ;[0.15 0.15 0.15 0.5] Painting rotation logic, both left and right
  ;;[0.15 0.15 0.15 0.5] If the puzzle has not been completed
  (if (not (Variables|Default|GetPuzzleComplete))
    (Utilities|FlowControl|Sequence
      (:then_0
        ;;[0.15 0.15 0.15 0.5] If the right interactor was chosen
        (if (Variables|/Game/Selectable/Static/BP_ItemInteractionSpot.BP_ItemInteractionSpot_C|GetItemPlaced (Utilities|Array|Get(acopy) (Variables|Default|GetPuzzleElements)))
          (CallFunction|RemovePuzzleElements)
          (Variables|Default|SetPuzzleComplete true)
          ;;[0.15 0.15 0.15 0.5] Bring the painting forward
          (bind (_direction _newtrack_0 _newtrack_1) (Timeline|MovePaintng PlayFromStart)
            (:Update
              (CallFunction|MovePaintingForward _newtrack_0)
              ;;[0.15 0.15 0.15 0.5] Rotate the painting 180 degrees to the right
              (Transformation|SetWorldRotation (Variables|Default|GetBP_queen_vic_painting) (Math|Rotator|Lerp(Rotator) "0.000000,90.000000,0.000000" "0.000000,-90.000000,0.000000" _newtrack_1) false false))
            (:Finished
              ;;[0.15 0.15 0.15 0.5] Move the painting back, now rotated
              (bind _newtrack_0_2 (Timeline|MovePaintingBack PlayFromStart)
                (:Update
                  (CallFunction|MovePaintingBackward _newtrack_0_2)))))))
      (:then_1
        ;;[0.15 0.15 0.15 0.5] If the left interactor was chosen
        (if (Variables|/Game/Selectable/Static/BP_ItemInteractionSpot.BP_ItemInteractionSpot_C|GetItemPlaced (Utilities|Array|Get(acopy) (Variables|Default|GetPuzzleElements) 1))
          (CallFunction|RemovePuzzleElements)
          (Variables|Default|SetPuzzleComplete true)
          ;;[0.15 0.15 0.15 0.5] Bring the painting forward
          (bind (_direction_2 _newtrack_0_3 _newtrack_1_2) (Timeline|Timeline PlayFromStart)
            (:Update
              (CallFunction|MovePaintingForward _newtrack_0_3)
              ;;[0.15 0.15 0.15 0.5] Rotate the painting 180 degrees to the left
              (Transformation|SetWorldRotation (Variables|Default|GetBP_queen_vic_painting) (Math|Rotator|Lerp(Rotator) "0.000000,90.000000,0.000000" "0.000000,270.000000,0.000000" _newtrack_1_2) false false))
            (:Finished
              ;;[0.15 0.15 0.15 0.5] Move the painting back now rotated
              (bind _newtrack_0_4 (Timeline|Timeline_0 PlayFromStart)
                (:Update
                  (CallFunction|MovePaintingBackward _newtrack_0_4))))))))))

(event EventBeginPlay
  ;[0.15 0.15 0.15 0.5] Set intial values
  (Utilities|FlowControl|Delay 0.2)
  (CallFunction|RemovePuzzleElements)
  (Variables|Default|SetInitialPosition (Transformation|GetWorldLocation (Variables|Default|GetBP_queen_vic_painting))))

(event EventOnSelectAdditional
  ;[0.15 0.15 0.15 0.5] When selected, if the puzzle hasn't been completed add the interactors
  (if (not (Variables|Default|GetPuzzleComplete))
    (CallFunction|AddPuzzleElements)))

(event EventOnDeSelect
  ;[0.15 0.15 0.15 0.5] When not selected remove the interactors
  (CallFunction|RemovePuzzleElements))

(fn ConstructionScript
  (|CallParentFunction))

(fn MovePaintingForward
  (params (Time :type Float%20%28single-precision%29))
  (Transformation|SetWorldLocation (Variables|Default|GetBP_queen_vic_painting) (Math|Vector|Lerp(Vector) (Variables|Default|GetInitialPosition) (Transformation|GetWorldLocation (Variables|Default|GetPaintingMoveTo)) Time) false false))

(fn MovePaintingBackward
  (params (Time :type Float%20%28single-precision%29))
  (Transformation|SetWorldLocation (Variables|Default|GetBP_queen_vic_painting) (Math|Vector|Lerp(Vector) (Transformation|GetWorldLocation (Variables|Default|GetPaintingMoveTo)) (Variables|Default|GetInitialPosition) Time) false false))